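; Player character Blueprint with a Fire function that plays a firing montage and runs two debug-drawn visibility traces.
; The first trace deprojects the viewport center and reaches a short fixed distance to find the aim point.
; The second runs from the mesh transform, with no socket named, to that hit location without checking for a hit.
; Its result is unused, and the event graph is empty.
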(event EventBeginPlay)

(event Collision|EventActorBeginOverlap
  (params (OtherActor :type Actor%20Object%20Reference)))

(event EventTick
  (params (DeltaSeconds :type Float%20%28single-precision%29)))

(fn ConstructionScript)

(fn Fire
  (bind _returnvalue (Game|GetPlayerController 0))
  (bind _returnvalue_2 (Viewport|GetViewportSize))
  (bind _returnvalue_3 (/ (.y _returnvalue_2) 2.0))
  (bind _returnvalue_4 (/ (.x _returnvalue_2) 2.0))
  (bind (_worldposition _worlddirection) (Class|GameplayStatics|DeprojectScreentoWorld _returnvalue (Math|Vector2D|MakeVector2D _returnvalue_4 _returnvalue_3)))
  (Animation|PlayAnimMontage "/Game/Animations/AM_Fire.AM_Fire" 1.0 "Default")
  (bind _outhit (Collision|LineTraceByChannel _worldposition (+ _worldposition (* _worlddirection 1e+03)) "TraceTypeQuery1" false 0 "ForDuration"))
  (Collision|LineTraceByChannel (.location (Transformation|GetSocketTransform (Variables|Character|GetMesh) "None" "RTS_World")) (.Location (Collision|BreakHitResult _outhit)) "TraceTypeQuery1" false 0 "ForDuration"))