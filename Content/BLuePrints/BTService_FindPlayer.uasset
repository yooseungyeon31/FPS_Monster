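; Behavior tree service that detects whether the player is near the AI-controlled pawn and records it in the Blackboard.
; On activation it waits briefly, then finds and caches the BP_Player actor.
; Each tick it checks straight-line distance to that actor, setting the Player key when within a fixed radius and clearing it otherwise, with no line-of-sight test.
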(event EventReceiveActivationAI
  (params (OwnerController :type AI%20Controller%20Object%20Reference) (ControlledPawn :type Pawn%20Object%20Reference))
  (Utilities|FlowControl|Delay 0.2)
  (bind _returnvalue (Actor|GetActorOfClass "/Game/BLuePrints/BP_Player.BP_Player_C"))
  (Variables|Default|SetBPPlayer _returnvalue))

(event EventReceiveTickAI
  (params (OwnerController :type AI%20Controller%20Object%20Reference) (ControlledPawn :type Pawn%20Object%20Reference) (DeltaSeconds :type Float%20%28single-precision%29))
  (Utilities|IsValid (Variables|Default|GetBPPlayer)
    (:Is%20Valid
      (if (< (Math|Vector|VectorLength (- (Transformation|GetActorLocation (Variables|Default|GetBPPlayer)) (Transformation|GetActorLocation ControlledPawn))) 1e+03)
        (Class|BTFunctionLibrary|SetBlackboardValueasObject (Variables|Default|GetPlayer) (Variables|Default|GetBPPlayer))
        (else
          (Class|BTFunctionLibrary|SetBlackboardValueasObject (Variables|Default|GetPlayer)))))))